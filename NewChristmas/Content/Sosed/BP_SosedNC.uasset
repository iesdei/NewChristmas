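; BP_SosedNC is the Neighbor AI in Hello Neighbor, with Mixer viewer buttons that toggle the generator's electricity or make him fall, each with a cooldown and popup widget.
; BeginPlay raises Easy difficulty to Hard.
; State changes control visibility, play attack music or fade it out by looping timer, and on Hunt trigger a throttled check of a nearby bed or cupboard.
; Tick tracks human visibility during Attack.
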(event `self.ReceiveBeginPlay`
  (`parent.ReceiveBeginPlay`)
  (bind _ashello_neighbor_game_instance (cast `HelloNeighborGameInstance` (`GameplayStatics.GetGameInstance`)))
  (bind (_returnvalue_m_elanguage _returnvalue_m_estartmap _returnvalue_m_fsensivitymouse _returnvalue_m_controllerstyle _returnvalue_m_binvertmousey _returnvalue_m_eneighborlevel) (break `GameParams` (`HelloNeighborGameInstance.GetGameParams` _ashello_neighbor_game_instance)))
  (if (`|EnumEquality` _returnvalue_m_eneighborlevel "Easy")
    (`HelloNeighborGameInstance.SetNeighborLevel` _ashello_neighbor_game_instance "Hard")))

(event `self.OnChangeState`
  (params (State :type "ENeighborState Enum" :default "NS_IDLE"))
  (bind _attack_sound (`self.attack_sound`))
  (bind _actors (`self.Actors`))
  (switch `ENeighborState` State
    (:`NS_IDLE`
      (`self.SetActorHiddenInGame` false :!label _label)
      (if (`AudioComponent.IsPlaying` (`self.attack_sound`))
        (bind _returnvalue (`KismetSystemLibrary.K2_SetTimerDelegate` (delegate `TimerSound`) 0.05 true))
        (set `self.Sound` _returnvalue)))
    (:`NS_HUNT`
      (`|ExecutionSequence`
        (:`then_0`
          (goto _label))
        (:`then_1`
          (bind _outactors (`GameplayStatics.GetAllActorsOfClass` "/Game/Objects/BP_Objects/BP_TwinBed.BP_TwinBed_C"))
          (bind _output_get (set `self.Actors` _outactors))
          (bind _outactors_2 (`GameplayStatics.GetAllActorsOfClass` "/Script/HelloNeighbor.Cupboard"))
          (`KismetArrayLibrary.Array_Append` _output_get _outactors_2)
          (for _array_element _actors
            (if (<= (`self.GetDistanceTo` _array_element) 700.0)
              (`/Engine/EditorBlueprintResources/StandardMacros.DoOnce` false :!label _label_2
                (:`Completed`
                  (`self.TutorialCheckObject` _array_element)
                  (`KismetSystemLibrary.PrintString` (`KismetSystemLibrary.GetDisplayName` _array_element))))))
          (`KismetArrayLibrary.Array_Clear` _actors)
          (`KismetSystemLibrary.Delay` 15.0)
          (goto _label_2 :!via `Reset`))))
    (:`NS_ATTACK`
      (`self.SetActorHiddenInGame` false)
      (if (`AudioComponent.IsPlaying` _attack_sound)
        (set `self.NeedPlay` true)
        (else
          (`AudioComponent.Play` _attack_sound 0.0))))
    (:`NS_DEMO`
      (`self.SetActorHiddenInGame` true)
      (goto _label))))

(event `TimerSound`
  (bind _attack_sound (`self.attack_sound`))
  (bind _returnvalue (- (`AudioComponent.VolumeMultiplier` _attack_sound) (* 0.05 0.3)))
  (if (< _returnvalue 0.0)
    (`AudioComponent.Stop` _attack_sound)
    (`AudioComponent.SetVolumeMultiplier` _attack_sound 1.0)
    (`KismetSystemLibrary.K2_ClearAndInvalidateTimerHandle` (`self.Sound`))
    (if (`self.NeedPlay`)
      (if (`|EnumEquality` (`self.GetState`) "NS_ATTACK")
        (`AudioComponent.Play` (`self.attack_sound`) 0.0))
      (set `self.NeedPlay` false))
    (else
      (`AudioComponent.SetVolumeMultiplier` _attack_sound _returnvalue))))

(event `self.ReceiveTick`
  (params (DeltaSeconds :type "Float (single-precision)"))
  (if (`|EnumEquality` (`self.GetState`) "NS_ATTACK")
    (`|ExecutionSequence`
      (:`then_1`
        (if (`self.IsVisibleHuman`)
          (set `self.boom2` 0.0)
          (elif (not (< (`self.boom`) (`self.boom2`)))
            (`self.SetState` "NS_ATTACK")
            (set `self.boom` (+ (`self.boom`) DeltaSeconds))))))))

(fn `UserConstructionScript`
  (`parent.UserConstructionScript`))
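; BP_HumanNC is the human player Blueprint for a Hello Neighbor game, adding inventory, cursor and trap widgets on BeginPlay.
; A 0.2-second loop forces power throw on and other abilities off.
; The SettingsNC save's UiMode hides cursor and inventory, reapplied by Update and after removing the post-save loading icon.
; Bound delegates cancel throws on the use key and teleport the player to the first PlayerStart on game-mode refresh.
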(event `self.ReceiveBeginPlay`
  (bind _ashello_neighbor_game_instance (cast `HelloNeighborGameInstance` (`GameplayStatics.GetGameInstance`))
    (:`then`
      (set `self.GameInstanceNew` _ashello_neighbor_game_instance)
      (bind _returnvalue (`|CreateWidget` "/Game/UMG/Inventory/BP_Inventory.BP_Inventory_C"))
      (bind _output_get (set `self.m_pInventory` _returnvalue))
      (`UserWidget.AddToViewport` _output_get 0)
      (bind _returnvalue_2 (`|CreateWidget` "/Game/UMG/Trap/BP_WidgetHumanInTrap.BP_WidgetHumanInTrap_C"))
      (set `self.TrapWidget` _returnvalue_2)
      (bind _returnvalue_3 (`|CreateWidget` "/Game/UMG/Cursor/BP_Cursor.BP_Cursor_C"))
      (bind _output_get_2 (set `self.m_pCursor` _returnvalue_3))
      (`UserWidget.AddToViewport` _output_get_2 0)
      (bind _returnvalue_4 (`self.IsLastPressGamepadKey`))
      (set `self.GamePad?` _returnvalue_4)
      (bind _ashello_neighbor_reborn_game_mode (cast `HelloNeighborRebornGameMode` (`GameplayStatics.GetGameMode`)))
      (add `HelloNeighborRebornGameMode.OnRefreshDelegate` _ashello_neighbor_reborn_game_mode (delegate `RefreshFix`))
      (`|ExecutionSequence`
        (:`then_0`
          (if (`self.AllScreenMessage`)
            (`KismetSystemLibrary.Delay` 3.0)
            (`KismetSystemLibrary.ExecuteConsoleCommand` "Enableallscreenmessages" null)
            (else
              (`KismetSystemLibrary.ExecuteConsoleCommand` "disableallscreenmessages" null))))
        (:`then_1`
          (add `self.OnInputPress` (delegate `CancelThrow`))
          (bind _ashello_neighbor_reborn_game_mode_2 (cast `HelloNeighborRebornGameMode` (`GameplayStatics.GetGameMode`)))
          (add `HelloNeighborRebornGameMode.OnPostSave` _ashello_neighbor_reborn_game_mode_2 (delegate `Delete`)))
        (:`then_2`
          (`self.SetDoubleJump` false :!label _label)
          (`self.SetEvade` false)
          (`self.SetEmission` false)
          (`self.SetInvisibility` false)
          (`self.SetPowerThrow` true)
          (`KismetSystemLibrary.Delay` 0.2)
          (goto _label))
        (:`then_3`
          (`KismetSystemLibrary.Delay` 0.0 :!label _label_2)
          (bind _returnvalue_5 (`GameplayStatics.LoadGameFromSlot` "SettingsNC"))
          (bind _asbp_saves_nc (cast `/NewChristmas/BP/Saves/BP_SavesNC` _returnvalue_5))
          (if (`/NewChristmas/BP/Saves/BP_SavesNC.UiMode` _asbp_saves_nc)
            (`self.SetVisibleCursor` "Hidden")
            (`self.SetVisibleInventory` "Hidden")
            (else
              (`self.SetVisibleCursor` "Visible")
              (`self.SetVisibleInventory` "Visible"))))))
    (:`CastFailed`
      (`KismetSystemLibrary.PrintString` "GameInstance not set in HUMAN"))))

(event `Delete`
  (bind _returnvalue (`GameplayStatics.LoadGameFromSlot` "SettingsNC"))
  (bind _asbp_saves_nc (cast `/NewChristmas/BP/Saves/BP_SavesNC` _returnvalue))
  (if (`/NewChristmas/BP/Saves/BP_SavesNC.UiMode` _asbp_saves_nc)
    (bind _foundwidgets (`WidgetBlueprintLibrary.GetAllWidgetsOfClass` "/Game/UMG/BPW_LoadingIcon.BPW_LoadingIcon_C"))
    (bind _output (`|GetArrayItem` _foundwidgets))
    (`/Engine/EditorBlueprintResources/StandardMacros.IsValid` _output
      (:`Is Valid`
        (`KismetSystemLibrary.Delay` 0.0)
        (`Widget.RemoveFromParent` _output)
        (goto _label_2)))))

(event `CancelThrow` :!signature `self.OnInputPress`
  (params (Key :type "Key Structure"))
  (bind (_returnvalue_name _returnvalue_action _returnvalue_typepress _returnvalue_key) (break `InputData` (`HelloNeighborGameInstance.GetInputActionInfo` (`self.GameInstanceNew`) "InputUse" (select `bool` (`self.GamePad?`) :`false` "Keyboard" :`true` "Gamepad" :!type "ETypeControl Enum"))))
  (if (and (== Key _returnvalue_key) (`|EnumEquality` (`self.GetHandsState`) "HS_SWEEP"))
    (`self.SetHandsState` "HS_CANCELTHROW")
    (`KismetSystemLibrary.Delay` 0.0)
    (`self.SetHandsState` "HS_HOLD")))

(event `RefreshFix`
  (bind _outactors (`GameplayStatics.GetAllActorsOfClass` "/Script/Engine.PlayerStart"))
  (`self.K2_SetActorLocation` (`self.K2_GetActorLocation` (`|GetArrayItem` _outactors)) false true))

(event `Update`
  (goto _label_2))

(fn `SetVisibleInventory`
  (params (Visible :type "ESlateVisibility Enum" :default "Visible"))
  (`Widget.SetVisibility` (`self.m_pInventory`) Visible))

(fn `UserConstructionScript`
  (`parent.UserConstructionScript`))
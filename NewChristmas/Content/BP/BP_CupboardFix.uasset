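; BP_CupboardFix is an interactive cupboard with Right and Left door components that open and close together.
; Interacting with either door reverses the door state, even mid-motion, unless the human found by FindHuman is in the MANTRAP state.
; State changes drive both doors' moving states and play open or close sounds, while the Right door's completion sets the final state.
; The construction script poses both doors to match the initial state.
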(event `self.OnEventAction`
  (params (ActionMaker :type "Actor Object Reference") (SpecialComponent :type "PrimitiveComponent Object Reference"))
  ;[1 1 1] Comment
  (bind _returnvalue (`Human.FindHuman`))
  (if (and (or (== SpecialComponent (`self.Right`)) (== SpecialComponent (`self.Left`))) (not (`|EnumEquality` (`Human.GetState` _returnvalue) "ES_MANTRAP")))
    (switch `EDoorState` (`self.GetDoorState`)
      (:`DS_OPEN`
        (`self.SetDoorState` "DS_CLOSING" :!label _label))
      (:`DS_CLOSING`
        (`self.SetDoorState` "DS_OPENING" :!label _label_2))
      (:`DS_CLOSE`
        (goto _label_2))
      (:`DS_OPENING`
        (goto _label)))))

(event `self.OnChangeDoorState`
  (params (NewState :type "EDoorState Enum" :default "DS_OPEN"))
  (bind _right (`self.Right`))
  (bind _left (`self.Left`))
  ;[1 1 1] Comment
  (switch `EDoorState` NewState
    (:`DS_CLOSING`
      (`AudioComponent.Play` (`self.wood_cupboard_closed_Cue`) 0.0)
      (`MovingComponent.SetMovingState` _right "MS_CLOSING")
      (`MovingComponent.SetMovingState` _left "MS_CLOSING"))
    (:`DS_OPENING`
      (`AudioComponent.Play` (`self.wood_cupboard_open_Cue`) 0.0)
      (`MovingComponent.SetMovingState` _right "MS_OPENING")
      (`MovingComponent.SetMovingState` _left "MS_OPENING"))))

(event `self.Right.OnChangeMovingState`
  (params (NewState :type "EMovingState Enum" :default "MS_OPEN"))
  (switch `EMovingState` NewState
    (:`MS_OPEN`
      (`self.SetDoorState` "DS_OPEN"))
    (:`MS_CLOSE`
      (`self.SetDoorState` "DS_CLOSE"))))

(fn `OnIsActionComponent`
  (params (Component :type "PrimitiveComponent Object Reference"))
  (returns (Result :type Boolean))
  (return (or (== Component (`self.Right`)) (== Component (`self.Left`)))))

(fn `UserConstructionScript`
  (bind _right (`self.Right`))
  (bind _left (`self.Left`))
  (switch `EDoorState` (`self.GetDoorState`)
    (:`DS_OPEN`
      (`MovingComponent.SetMovingState` _right "MS_OPEN")
      (`MovingComponent.SetMovingState` _left "MS_OPEN"))
    (:`DS_CLOSE`
      (`MovingComponent.SetMovingState` _right "MS_CLOSE")
      (`MovingComponent.SetMovingState` _left "MS_CLOSE"))))
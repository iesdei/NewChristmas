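; Hammer item that pulls out nails and can sit fixed in a holder as its crowbar.
; Applying it to a Nail plays timed sounds with repeated range checks, then ejects the nail or plays a fallback sound.
; SetHolder fixes its FlatComponent, a hit frees it, and save/load tracks the holder, clearing it when none was saved.
; Temperature crossing zero swaps materials, using dynamic instances when hot; the construction script sets initial materials.
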(event `self.ReceiveBeginPlay`
  (bind _returnvalue (`KismetMaterialLibrary.CreateDynamicMaterialInstance` "/Game/Objects/Materials/instances/Hot_Material/metal_noise_hot_Inst.metal_noise_hot_Inst"))
  (bind _returnvalue_2 (`KismetMaterialLibrary.CreateDynamicMaterialInstance` "/Game/Objects/Materials/instances/Hot_Material/red_dark_hot_Inst.red_dark_hot_Inst"))
  (set `self.MaterialsHot` (`|MakeArray` _returnvalue _returnvalue_2)))

(event `self.OnLoad`
  (params (JsonObject :type "JSON Structure"))
  ;[1 1 1] Загрузка из сохранки
  (bind (_stringvalue _returnvalue) (`JSONLibrary.GetValueAsString` JsonObject "Holder"))
  (if _returnvalue
    _
    (elif (`KismetSystemLibrary.IsValid` (`self.Holder`))
      (set `/Game/Objects/BP_Objects/BP_ElectricWires.Crowbar` null (`self.Holder`))
      (set `self.Holder` null)
      (`FlatComponent.SetMode` (`self.FlatComponent`) "FM_Suspend"))))

(event `self.OnPostLoad`
  ;[1 1 1] После загрузки
  (`self.ChangeMaterial`))

(event `self.OnChangeTemperature`
  (params (Old :type "Float (single-precision)") (New :type "Float (single-precision)"))
  ;[1 1 1] Изменения температуры
  (if (or (and (> Old 0.0) (<= New 0.0)) (and (<= Old 0.0) (> New 0.0)))
    (`self.ChangeMaterial`)))

(event `self.ReceiveHit`
  (params (MyComp :type "PrimitiveComponent Object Reference") (Other :type "Actor Object Reference") (OtherComp :type "PrimitiveComponent Object Reference") (bSelfMoved :type Boolean) (HitLocation :type "Vector Structure") (HitNormal :type "Vector Structure") (NormalImpulse :type "Vector Structure") (Hit :type "HitResult Structure (by ref)"))
  ;[1 1 1] Ударился или в него попали чем-то
  (if (`KismetSystemLibrary.IsValid` (`self.Holder`))
    (`FlatComponent.SetMode` (`self.FlatComponent`) "FM_Free")
    (set `/Game/Objects/BP_Objects/BP_ElectricWires.Crowbar` null (`self.Holder`))
    (set `self.Holder` null)))

(event `ChangeMaterial`
  (bind _staticmeshcomponent (`self.StaticMeshComponent`))
  ;[1 1 1] Изменить метериал
  (if (<= (`self.GetTemperature`) 0.0)
    (`PrimitiveComponent.SetMaterial` _staticmeshcomponent 0 "/Game/Objects/Materials/instances/Hot_Material/metal_noise_hot_Inst.metal_noise_hot_Inst")
    (`PrimitiveComponent.SetMaterial` _staticmeshcomponent 1 "/Game/Objects/Materials/instances/Hot_Material/red_dark_hot_Inst.red_dark_hot_Inst")
    (else
      (`PrimitiveComponent.SetMaterial` _staticmeshcomponent 0 (`|GetArrayItem` (`self.MaterialsHot`)))
      (`PrimitiveComponent.SetMaterial` _staticmeshcomponent 1 (`|GetArrayItem` (`self.MaterialsHot`) 1)))))

(event `self.Apply.OnApply`
  (params (ApplyActor :type "Actor Object Reference") (TraceActor :type "FlatActor Object Reference") (TraceComponent :type "PrimitiveComponent Object Reference"))
  (bind _asnail (cast `Nail` TraceActor))
  (`KismetSystemLibrary.Delay` 0.8)
  (if (<= (`self.GetDistanceTo` _asnail) 150.0)
    (`GameplayStatics.PlaySound2D` "/NewChristmas/Sounds/Hammer_use_01.Hammer_use_01" 1.0 1.0 0.0 null null)
    (`KismetSystemLibrary.Delay` 0.32)
    (`GameplayStatics.PlaySound2D` "/NewChristmas/Sounds/Hammer_use_02.Hammer_use_02" 1.0 1.0 0.0 null null)
    (if (<= (`self.GetDistanceTo` _asnail) 150.0)
      (`KismetSystemLibrary.Delay` 0.67)
      (`GameplayStatics.PlaySound2D` "/NewChristmas/Sounds/Hammer_use_03.Hammer_use_03" 1.0 1.0 0.0 null null)
      (if (<= (`self.GetDistanceTo` _asnail) 150.0)
        (`Nail.Eject` _asnail)
        (else
          (`GameplayStatics.PlaySound2D` "/NewChristmas/Sounds/SN_unblock_ended.SN_unblock_ended" 1.0 1.0 0.0 null null :!label _label)))
      (else
        (goto _label)))
    (else
      (goto _label))))

(event `self.OnGrab`
  (params (Character :type "Actor Object Reference"))
  (`self.WasTaken`))

(fn `OnIsActionComponent`
  (params (Component :type "PrimitiveComponent Object Reference"))
  (returns (Result :type Boolean))
  (return true))

(fn `OnSave`
  (params (JsonObject :type "JSON Structure"))
  (if (`KismetSystemLibrary.IsValid` (`self.Holder`))
    (`JSONLibrary.SetValueAsString` JsonObject "Holder" (`KismetSystemLibrary.GetDisplayName` (`self.Holder`)))))

(fn `SetHolder`
  (params (Holder :type "/Game/Objects/BP_Objects/BP_ElectricWires Object Reference"))
  (bind _output_get (set `self.Holder` Holder))
  (if (`KismetSystemLibrary.IsValid` _output_get)
    (`FlatComponent.SetMode` (`self.FlatComponent`) "FM_Fixed")))

(fn `UserConstructionScript`
  (bind _staticmeshcomponent (`self.StaticMeshComponent`))
  (if (<= (`self.GetTemperature`) 0.0)
    (`PrimitiveComponent.SetMaterial` _staticmeshcomponent 0 "/Game/Objects/Materials/instances/metal_noise_dark_Inst.metal_noise_dark_Inst")
    (`PrimitiveComponent.SetMaterial` _staticmeshcomponent 1 "/Game/Objects/Materials/instances/red_dark_wood_Inst.red_dark_wood_Inst")
    (`PrimitiveComponent.SetMaterial` _staticmeshcomponent 2 "/Game/Objects/Materials/instances/metal_noise_Inst.metal_noise_Inst")
    (else
      (`PrimitiveComponent.SetMaterial` _staticmeshcomponent 0 "/Game/Objects/Materials/instances/metal_hot_Inst.metal_hot_Inst")
      (`PrimitiveComponent.SetMaterial` _staticmeshcomponent 1 "/Game/Objects/Materials/instances/metal_hot_Inst.metal_hot_Inst")
      (`PrimitiveComponent.SetMaterial` _staticmeshcomponent 2 "/Game/Objects/Materials/instances/metal_hot_Inst.metal_hot_Inst")
      (`MeshComponent.SetScalarParameterValueOnMaterials` (`self.StaticMeshComponent`) "temperature" (* (`self.GetTemperature`) 15.0)))))
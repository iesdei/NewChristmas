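; BP_CrowbarRemade is a crowbar actor that opens a gate when applied to a wire-need object.
; Its Apply.OnApply event continues only for a BP_WireNeed target and fires once through a DoOnce.
; It then plays a metal rattle sound, sets the referenced Gate's platform moving state to open and hides the referenced Actor.
; Every component counts as an action component, while OnActionApply and GetLight are empty.
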(event `self.OnActionApply`
  (params (HitActor :type "Actor Object Reference")))

(event `self.Apply.OnApply`
  (params (ApplyActor :type "Actor Object Reference") (TraceActor :type "FlatActor Object Reference") (TraceComponent :type "PrimitiveComponent Object Reference"))
  (cast `/NewChristmas/BP/BP_WireNeed` ApplyActor)
  (`/Engine/EditorBlueprintResources/StandardMacros.DoOnce` false
    (:`Completed`
      (`GameplayStatics.PlaySound2D` "/Game/Sounds/Maps/Act2/Main/metal_rattle_blok_Cue.metal_rattle_blok_Cue" 1.0 1.0 0.0 null null)
      (`MovingComponent.SetMovingState` (`/Game/Objects/BP_Objects/BP_PlatformDoor.Platform` (`self.Gate`)) "MS_OPEN")
      (`self.SetActorHiddenInGame` (`self.Actor`) true))))

(fn `GetLight`
  (returns (Light :type "LightComponent Object Reference"))
  (return null))

(fn `OnIsActionComponent`
  (params (Component :type "PrimitiveComponent Object Reference"))
  (returns (Result :type Boolean))
  (return true))

(fn `UserConstructionScript`)
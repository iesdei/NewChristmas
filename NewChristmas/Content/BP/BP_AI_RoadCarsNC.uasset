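; BP_AI_RoadCarsNC controls road traffic by periodically sending idle cars from its Cars list on their way.
; On Tick it checks its Box for overlapping BP_Human actors and freezes the countdown while any are inside.
; When the randomized pause runs out, it starts the first stationary car in the direction opposite to its current one, so cars shuttle back and forth.
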(event `OnCarStopMove`
  (params (Car :type "/Game/Objects/BP_Objects/BP_RoadCar Object Reference")))

(event `self.ReceiveBeginPlay`)

(event `self.ReceiveTick`
  (params (DeltaSeconds :type "Float (single-precision)"))
  (bind _output_get (set `self.bPlayerInBox` (> (`KismetArrayLibrary.Array_Length` (`PrimitiveComponent.GetOverlappingActors` (`self.Box`) "/Game/Player/BP_Human.BP_Human_C")) 0)))
  (if _output_get
    _
    (elif (<= (`self.Timer`) 0.0)
      (set `self.Timer` (`KismetMathLibrary.RandomFloatInRange` (`self.PauseBetweenMin`) (`self.PauseBetweenMax`)))
      (for _array_element (`self.Cars`)
        (if (not (`RoadCar.IsMove` _array_element))
          (`RoadCar.StartMove` _array_element (not (`RoadCar.IsForwardDir` _array_element)))
          (break)))
      (else
        (set `self.Timer` (- (`self.Timer`) DeltaSeconds))))))

(fn `UserConstructionScript`)
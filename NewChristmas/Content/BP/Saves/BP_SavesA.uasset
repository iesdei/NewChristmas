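; BP_SavesA is a save-handling Blueprint that, on post-load, collects all FlatActors and loads the "SettingsNC" save, creating it first if missing.
; An unwired chain, which never runs, would restore each FlatActor's type-specific state, mode, transform or inventory slot from the indexed "SaveSlots" entry.
; That chain matches saved data by actor array index, reselects the inventory slot, then clears the pending-load flag.
; OnPreSave is empty.
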(event `self.OnPostLoad`
  (bind _outactors (`GameplayStatics.GetAllActorsOfClass` "/Script/HelloNeighbor.FlatActor"))
  (for _array_element _outactors
    (`KismetArrayLibrary.Array_Add` (`self.FlatActors`) _array_element))
  (bind _returnvalue (`GameplayStatics.DoesSaveGameExist` "SettingsNC"))
  (if (not _returnvalue)
    (bind _returnvalue_2 (`GameplayStatics.CreateSaveGameObject` "/NewChristmas/BP/Saves/BP_SavesNC.BP_SavesNC_C"))
    (`GameplayStatics.SaveGameToSlot` _returnvalue_2 "SettingsNC"))
  (`GameplayStatics.LoadGameFromSlot` "SettingsNC"))

(event `self.OnPreSave`)

(fn `UserConstructionScript`)
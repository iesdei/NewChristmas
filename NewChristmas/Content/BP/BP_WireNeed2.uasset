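; BP_WireNeed2 is a crowbar holder, apparently a wire puzzle piece, that opens a linked Gate when a crowbar is placed in it.
; HolderCrowbar snaps the crowbar to StaticMesh1, sets its FlatComponent to Fixed, flags Save and opens the Gate platform.
; That flag persists through JSON; on post-load, a set flag snaps every BP_CrowbarRemade2 to the holder and reopens the gate, otherwise it closes.
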(event `self.OnLoad`
  (params (JsonObject :type "JSON Structure"))
  (bind _boolvalue (`JSONLibrary.GetValueAsBool` JsonObject "s"))
  (bind _output_get (set `self.Save` _boolvalue))
  (`KismetSystemLibrary.PrintString` (`KismetStringLibrary.Conv_BoolToString` _output_get) true true (struct :`R` 1.0 :`B` 0.053367 :`A` 1.0) 25.0))

(event `self.OnPostLoad`
  (if (`self.Save`)
    (bind _outactors (`GameplayStatics.GetAllActorsOfClass` "/NewChristmas/BP/BP_CrowbarRemade2.BP_CrowbarRemade2_C"))
    (for _array_element _outactors
      (`self.K2_SetActorTransform` _array_element (`SceneComponent.K2_GetComponentToWorld` (`self.StaticMesh1`)) false true)
      (`FlatComponent.SetMode` (`FlatActor.FlatComponent` _array_element) "FM_Fixed")
      (`MovingComponent.SetMovingState` (`/Game/Objects/BP_Objects/BP_PlatformDoor.Platform` (`self.Gate`)) "MS_OPENING"))
    (else
      (`MovingComponent.SetMovingState` (`/Game/Objects/BP_Objects/BP_PlatformDoor.Platform` (`self.Gate`)) "MS_CLOSE"))))

(event `HolderCrowbar`
  (params (Crowbar :type "/NewChristmas/BP/BP_CrowbarRemade2 Object Reference"))
  (bind _output_get (set `self.Crowbar` Crowbar))
  (`KismetSystemLibrary.Delay` 0.0)
  (`self.K2_SetActorTransform` _output_get (`SceneComponent.K2_GetComponentToWorld` (`self.StaticMesh1`)) false true)
  (`FlatComponent.SetMode` (`FlatActor.FlatComponent` _output_get) "FM_Fixed")
  (set `self.Save` true)
  (`MovingComponent.SetMovingState` (`/Game/Objects/BP_Objects/BP_PlatformDoor.Platform` (`self.Gate`)) "MS_OPENING"))

(event `self.ReceiveTick`
  (params (DeltaSeconds :type "Float (single-precision)")))

(fn `OnIsActionComponent`
  (params (Component :type "PrimitiveComponent Object Reference"))
  (returns (Result :type Boolean))
  (return true))

(fn `OnSave`
  (params (JsonObject :type "JSON Structure"))
  (`JSONLibrary.SetValueAsBool` JsonObject "s" (`self.Save`)))

(fn `UserConstructionScript`)
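; BP_CutScene is a trigger actor that plays a level sequence cutscene when a BP_HumanNC enters its box.
; A DoOnce gate blocks repeat overlaps, and a long fixed delay precedes playback.
; When the sequence finishes, the Delete event waits a random interval and reopens the gate instead of destroying anything.
; The debug print rolls its own random number, so it does not show the actual wait.
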(event `self.Box.OnComponentBeginOverlap`
  (params (OverlappedComponent :type "PrimitiveComponent Object Reference") (OtherActor :type "Actor Object Reference") (OtherComp :type "PrimitiveComponent Object Reference") (OtherBodyIndex :type Integer) (bFromSweep :type Boolean) (SweepResult :type "HitResult Structure (by ref)"))
  (bind _sequenceplayer (`LevelSequenceActor.SequencePlayer` (`self.Cut-Scene`)))
  (cast `/NewChristmas/Player/BP_HumanNC` OtherActor)
  (`/Engine/EditorBlueprintResources/StandardMacros.DoOnce` false :!label _label
    (:`Completed`
      (`KismetSystemLibrary.Delay` 80.0)
      (`MovieSceneSequencePlayer.Play` _sequenceplayer)
      (add `MovieSceneSequencePlayer.OnFinished` _sequenceplayer (delegate `Delete`)))))

(event `Delete`
  (bind _returnvalue (`KismetMathLibrary.RandomFloatInRange` 60.0 360.0))
  (`KismetSystemLibrary.Delay` _returnvalue)
  (`KismetSystemLibrary.PrintString` (`KismetStringLibrary.Conv_DoubleToString` _returnvalue))
  (goto _label :!via `Reset`))

(fn `UserConstructionScript`)
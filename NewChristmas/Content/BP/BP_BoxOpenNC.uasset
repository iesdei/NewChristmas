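; Open 150 kg carryable box that takes loose physics FlatActors inside it along when picked up.
; While not grabbed, a slowed Tick rescans the overlap volume and adds mesh components marking each item's relative transform.
; Grab attaches items at those markers without collision, throw frees them, and Tick hides them while the box is in inventory.
; Save stores grab state, display names and locations as strings, which load uses to reattach items.
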(event `self.Box.OnComponentBeginOverlap`
  (params (OverlappedComponent :type "PrimitiveComponent Object Reference") (OtherActor :type "Actor Object Reference") (OtherComp :type "PrimitiveComponent Object Reference") (OtherBodyIndex :type Integer) (bFromSweep :type Boolean) (SweepResult :type "HitResult Structure (by ref)")))

(event `self.ReceiveBeginPlay`
  (`PrimitiveComponent.SetMassOverrideInKg` (`self.StaticMeshComponent`) "None" 150.0 true)
  (`self.SetActorTickInterval` 0.2))

(event `self.OnPreSave`
  (for _array_element (`self.FlatActors`)
    (set `self.StringObjects` (`KismetStringLibrary.BuildString_Name` (`self.StringObjects`) " \n" (`KismetStringLibrary.Conv_StringToName` (`KismetSystemLibrary.GetDisplayName` _array_element))))
    (set `self.StringLocation` (`KismetStringLibrary.BuildString_Vector` (`self.StringLocation`) " \n" (`self.K2_GetActorLocation` _array_element))))
  (`KismetSystemLibrary.Delay` 0.5)
  (set `self.StringObjects` "")
  (set `self.StringLocation` ""))

(event `self.OnLoad`
  (params (JsonObject :type "JSON Structure"))
  (bind _flatactors (`self.FlatActors`))
  (bind _boolvalue (`JSONLibrary.GetValueAsBool` JsonObject "PickUp"))
  (bind _output_get (set `self.Pow` _boolvalue))
  (if _output_get
    (bind _stringvalue (`JSONLibrary.GetValueAsString` JsonObject "Objects"))
    (bind _output_get_2 (set `self.StringObjects` _stringvalue))
    (bind _output_get_3 (set `self.StringObjectsArray` (`KismetStringLibrary.ParseIntoArray` _output_get_2 " \n" false)))
    (`KismetArrayLibrary.Array_Remove` _output_get_3)
    (bind _stringvalue_2 (`JSONLibrary.GetValueAsString` JsonObject "Loc"))
    (bind _output_get_4 (set `self.StringLocationArray` (`KismetStringLibrary.ParseIntoArray` _stringvalue_2 " \n" false)))
    (`KismetArrayLibrary.Array_Remove` _output_get_4)
    (for _array_element _output_get_4
      (`KismetArrayLibrary.Array_Add` (`self.Location`) (`KismetStringLibrary.Conv_StringToVector` _array_element)))
    (bind _outactors (`GameplayStatics.GetAllActorsOfClass` "/Script/HelloNeighbor.FlatActor"))
    (for (_array_element_2 _array_index) _outactors
      (if (not (== (`KismetArrayLibrary.Array_Find` (`self.StringObjectsArray`) (`KismetSystemLibrary.GetDisplayName` _array_element_2)) -1))
        (`KismetArrayLibrary.Array_Add` _flatactors _array_element_2)
        (bind _returnvalue (`AddComponent|NODE_AddStaticMeshComponent-3` :`RelativeTransform` (`KismetMathLibrary.MakeTransform` (`|GetArrayItem` (`self.Location`) _array_index))))
        (`KismetArrayLibrary.Array_Add` (`self.G`) _returnvalue)))
    (for (_array_element_3 _array_index_2) _flatactors
      (`FlatComponent.SetMode` (`FlatActor.FlatComponent` _array_element_3) "FM_Fixed")
      (`self.K2_AttachToComponent` _array_element_3 (`self.StaticMeshComponent`) "None" "KeepRelative" "KeepRelative" "KeepRelative" true)
      (`self.SetPickUp` _array_element_3 false)
      (`self.SetActorEnableCollision` _array_element_3 false)
      (`self.K2_SetActorLocation` _array_element_3 (`|GetArrayItem` (`self.Location`) _array_index_2) false false))))

(event `self.Box.OnComponentEndOverlap`
  (params (OverlappedComponent :type "PrimitiveComponent Object Reference") (OtherActor :type "Actor Object Reference") (OtherComp :type "PrimitiveComponent Object Reference") (OtherBodyIndex :type Integer)))

(event `self.ReceiveTick`
  (params (DeltaSeconds :type "Float (single-precision)"))
  (if (not (`self.Pow`))
    (`|ExecutionSequence`
      (:`then_0`
        (`KismetSystemLibrary.Delay` 0.0)
        (`KismetArrayLibrary.Array_Clear` (`self.FlatActors`))
        (`KismetArrayLibrary.Array_Clear` (`self.G`))
        (for _array_element (`PrimitiveComponent.GetOverlappingActors` (`self.Box`) "/Script/HelloNeighbor.FlatActor")
          (bind _asflat_actor (cast `FlatActor` _array_element))
          (bind _flatcomponent (`FlatActor.FlatComponent` _asflat_actor))
          (bind _mode (`FlatComponent.Mode` _flatcomponent))
          (if (and (`|EnumEquality` (`FlatComponent.Type` _flatcomponent) "FT_Physic") (!= _asflat_actor self) (or (`|EnumEquality` _mode "FM_Free") (`|EnumEquality` _mode "FM_Suspend")))
            (`KismetArrayLibrary.Array_Add` (`self.FlatActors`) _asflat_actor)
            (bind _returnvalue (`AddComponent|NODE_AddStaticMeshComponent-1` :`RelativeTransform` (`KismetMathLibrary.ComposeTransforms` (`self.GetTransform` _asflat_actor) (`KismetMathLibrary.InvertTransform` (`self.GetTransform`)))))
            (`KismetArrayLibrary.Array_Add` (`self.G`) _returnvalue))))
      (:`then_1`
        (for _array_element_2 (`self.FlatActors`) :!label _label
          (`/Engine/EditorBlueprintResources/StandardMacros.IsValid` _array_element_2
            (:`Is Valid`
              (`self.SetActorHiddenInGame` _array_element_2 (`|EnumEquality` (`FlatComponent.Mode` (`self.FlatComponent`)) "FM_Inventory")))))))
    (else
      (goto _label))))

(event `self.OnGrab`
  (params (Character :type "Actor Object Reference"))
  (set `self.Pow` true)
  (for (_array_element _array_index) (`self.FlatActors`)
    (`FlatComponent.SetMode` (`FlatActor.FlatComponent` _array_element) "FM_Fixed")
    (`self.K2_AttachToComponent` _array_element (`self.StaticMeshComponent`) "None" "KeepRelative" "KeepRelative" "KeepRelative" true)
    (`self.SetPickUp` _array_element false)
    (`self.SetActorEnableCollision` _array_element false)
    (`self.K2_SetActorTransform` _array_element (`SceneComponent.K2_GetComponentToWorld` (`|GetArrayItem` (`self.G`) _array_index)) false true)))

(event `self.OnThrow`
  (params (Character :type "Character Object Reference"))
  (set `self.Pow` false)
  (`KismetSystemLibrary.Delay` 0.0)
  (for _array_element (`self.FlatActors`)
    (bind _flatcomponent (`FlatActor.FlatComponent` _array_element))
    (bind _mode (`FlatComponent.Mode` _flatcomponent))
    (if (not (or (`|EnumEquality` _mode "FM_HumanHand") (`|EnumEquality` _mode "FM_Inventory")))
      (`FlatComponent.SetMode` _flatcomponent "FM_Free")
      (`self.K2_DetachFromActor` _array_element "KeepRelative" "KeepRelative" "KeepRelative")
      (`self.SetPickUp` _array_element true)
      (`self.SetActorEnableCollision` _array_element true))))

(fn `OnIsActionComponent`
  (params (Component :type "PrimitiveComponent Object Reference"))
  (returns (Result :type Boolean))
  (return true))

(fn `OnSave`
  (params (JsonObject :type "JSON Structure"))
  (`JSONLibrary.SetValueAsBool` JsonObject "PickUp" (`self.Pow`))
  (`JSONLibrary.SetValueAsString` JsonObject "Objects" (`self.StringObjects`))
  (`JSONLibrary.SetValueAsString` JsonObject "Loc" (`self.StringLocation`)))

(fn `UserConstructionScript`)
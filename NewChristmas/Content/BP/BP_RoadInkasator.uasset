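; BP_RoadInkasator is a road actor, apparently a cash-in-transit vehicle by its name, that awards an achievement when it hits a dummy.
; Its construction script applies the configurable Mesh to the static mesh component.
; On a hit with an actor of exactly the BP_Dummy class, a DoOnce writes the "Meet Joe Black" achievement through the HelloNeighborReborn game mode.
; Tick is empty, and no movement logic is defined here.
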(event `self.ReceiveHit`
  (params (MyComp :type "PrimitiveComponent Object Reference") (Other :type "Actor Object Reference") (OtherComp :type "PrimitiveComponent Object Reference") (bSelfMoved :type Boolean) (HitLocation :type "Vector Structure") (HitNormal :type "Vector Structure") (NormalImpulse :type "Vector Structure") (Hit :type "HitResult Structure (by ref)"))
  (`/Engine/EditorBlueprintResources/StandardMacros.IsValid` Other
    (:`Is Valid`
      (if (== (`GameplayStatics.GetObjectClass` Other) "/Game/Objects/BP_Objects/BP_Dummy.BP_Dummy_C")
        (`/Engine/EditorBlueprintResources/StandardMacros.DoOnce` false
          (:`Completed`
            ;[1 1 1] Ачивка
            (bind _ashello_neighbor_reborn_game_mode (cast `HelloNeighborRebornGameMode` (`GameplayStatics.GetGameMode`)))
            (`HelloNeighborRebornGameMode.WriteAchievements` _ashello_neighbor_reborn_game_mode "HNACH_MEET_JOE_BLACK" 100.0)))))))

(event `self.ReceiveTick`
  (params (DeltaSeconds :type "Float (single-precision)")))

(fn `UserConstructionScript`
  (bind _staticmesh (`self.StaticMesh`))
  (`/Engine/EditorBlueprintResources/StandardMacros.IsValid` _staticmesh
    (:`Is Valid`
      (`StaticMeshComponent.SetStaticMesh` _staticmesh (`self.Mesh`)))))
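; Interactable gramophone that toggles music and affects nearby tomato bushes while it plays.
; BeginPlay picks the good or alternative audio from IsGood, and action events on the body or vinyl start or stop it.
; While playing, Tick spins the vinyl and sphere-overlaps for BP_TomatoBush actors, passing IsGood to HearingMusic every frame, noted as driving their size change.
; The needle also reports as an action component but does not toggle playback.
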(event `self.ReceiveBeginPlay`
  (if (`self.IsGood`)
    (set `self.Music` (`self.AudioGood`))
    (else
      (set `self.Music` (`self.attack_gram_Cue`)))))

(event `self.ReceiveTick`
  (params (DeltaSeconds :type "Float (single-precision)"))
  (bind _sphere (`self.Sphere`))
  (if (`AudioComponent.IsPlaying` (`self.Music`))
    ;[1 1 1] Vinyl Spinning
    (`SceneComponent.K2_SetRelativeRotation` (`self.vinyl`) (`KismetMathLibrary.ComposeRotators` (`SceneComponent.RelativeRotation` (`self.vinyl`)) (`KismetMathLibrary.MakeRotator` 0.0 0.0 (`self.Speed`))) false true)
    ;[1 1 1] Эвент чтобы меняли размер
    (bind _outactors (`KismetSystemLibrary.SphereOverlapActors` (`SceneComponent.K2_GetComponentLocation` _sphere) (`SphereComponent.GetScaledSphereRadius` _sphere) (`|MakeArray` "ObjectTypeQuery1" :!type "EObjectTypeQuery Enum") "/Game/Objects/BP_Objects/Puzzles/BP_TomatoBush.BP_TomatoBush_C" (`|MakeArray` self :!type "Actor Object Reference")))
    (for _array_element _outactors
      (bind _asbp_tomato_bush (cast `/Game/Objects/BP_Objects/Puzzles/BP_TomatoBush` _array_element))
      (`/Game/Objects/BP_Objects/Puzzles/BP_TomatoBush.HearingMusic` _asbp_tomato_bush (`self.IsGood`)))))

(event `self.OnEventAction`
  (params (ActionMaker :type "Actor Object Reference") (SpecialComponent :type "PrimitiveComponent Object Reference"))
  (bind _music (`self.Music`))
  (if (or (== (`self.StaticMeshComponent`) SpecialComponent) (== SpecialComponent (`self.vinyl`)))
    (if (`AudioComponent.IsPlaying` (`self.Music`))
      (`AudioComponent.Stop` _music)
      (else
        (`AudioComponent.Play` _music 0.0)))))

(fn `OnIsActionComponent`
  (params (Component :type "PrimitiveComponent Object Reference"))
  (returns (Result :type Boolean))
  (return (or (== Component (`self.StaticMeshComponent`)) (== Component (`self.vinyl`)) (== Component (`self.niddle`)))))

(fn `UserConstructionScript`
  (`PrimitiveComponent.SetMaterial` (`self.StaticMeshComponent`) 0 "/NewChristmas/Materials/M_Multi_nc_Inst.M_Multi_nc_Inst"))
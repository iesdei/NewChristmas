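; BP_TrapNC is a trap Blueprint with a base mesh and five box components, including left, right and grab boxes.
; On BeginPlay it overrides the base mesh mass to make it heavy, then after a short delay sets all five boxes to ignore a custom trace channel.
; OnIsActionComponent reports every component as an action component.
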(event `self.ReceiveBeginPlay`
  ;[1 1 1] Comment
  (`PrimitiveComponent.SetMassOverrideInKg` (`self.BaseMesh`) "None" 1000.0 true)
  (`KismetSystemLibrary.Delay` 1.0)
  (`PrimitiveComponent.SetCollisionResponseToChannel` (`self.BoxLeft`) "ECC_GameTraceChannel2" "ECR_Ignore")
  (`PrimitiveComponent.SetCollisionResponseToChannel` (`self.BoxRight`) "ECC_GameTraceChannel2" "ECR_Ignore")
  (`PrimitiveComponent.SetCollisionResponseToChannel` (`self.BoxGrab`) "ECC_GameTraceChannel2" "ECR_Ignore")
  (`PrimitiveComponent.SetCollisionResponseToChannel` (`self.Box1`) "ECC_GameTraceChannel2" "ECR_Ignore")
  (`PrimitiveComponent.SetCollisionResponseToChannel` (`self.Box2`) "ECC_GameTraceChannel2" "ECR_Ignore"))

(fn `OnIsActionComponent`
  (params (Component :type "PrimitiveComponent Object Reference"))
  (returns (Result :type Boolean))
  (return true))

(fn `UserConstructionScript`)
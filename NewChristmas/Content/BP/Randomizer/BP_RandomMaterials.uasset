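; BP_RandomMaterials randomizes materials on referenced static mesh actors and persists the result through JSON save and load.
; While the Save flag is set, OnPostLoad picks a random material set and a material per mesh slot, encodes the indices into a string and clears the flag.
; Otherwise it parses the saved string back into indices.
; Both paths then apply the materials, printing each index for debugging.
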(event `self.OnLoad`
  (params (JsonObject :type "JSON Structure"))
  ;[0 0.09306 0.5583] упаковка
  (bind _intvalue (`JSONLibrary.GetValueAsInt` JsonObject "7"))
  (set `self.Int` _intvalue)
  (bind _boolvalue (`JSONLibrary.GetValueAsBool` JsonObject "8"))
  (set `self.Save` _boolvalue)
  (bind _intvalue_2 (`JSONLibrary.GetValueAsInt` JsonObject "9"))
  (set `self.Int2` _intvalue_2)
  (bind _stringvalue (`JSONLibrary.GetValueAsString` JsonObject "2"))
  (set `self.String` _stringvalue))

(event `self.OnPostLoad`
  (bind _intarray (`self.IntArray`))
  (bind _intarray_2 (`self.IntArray`))
  (bind _randommaterials (`self.RandomMaterials`))
  ;[1 1 1] Начальная генерация материалов
  (if (`self.Save`)
    (bind _output_get (set `self.Int` (`KismetMathLibrary.RandomIntegerInRange` 0 (`KismetArrayLibrary.Array_LastIndex` _randommaterials))))
    (bind _output_get_2 (set `self.ChosenMaterials` (`|GetArrayItem` _randommaterials _output_get)))
    (for _array_element (`.Random_3_FBC1B23240D51253641D7097DFDE1E31` (break `/NewChristmas/BP/Randomizer/S_PotentialMaterials` _output_get_2))
      (bind _output_get_3 (set `self.Int2` (`KismetMathLibrary.RandomIntegerInRange` 0 (`KismetArrayLibrary.Array_LastIndex` (`.Materials_10_81E0B3C0442D85CDEC0549B89F49BAC6` (break `/NewChristmas/BP/Randomizer/S_RandomMaterials` _array_element))))))
      (`PrimitiveComponent.SetMaterial` (`StaticMeshActor.StaticMeshComponent` (break `/NewChristmas/BP/Randomizer/S_RandomMaterials` _array_element)) (`.IndexMaterial_6_622B93D74E9D80B410BB6C940510CCFE` (break `/NewChristmas/BP/Randomizer/S_RandomMaterials` _array_element)) (`|GetArrayItem` (`.Materials_10_81E0B3C0442D85CDEC0549B89F49BAC6` (break `/NewChristmas/BP/Randomizer/S_RandomMaterials` _array_element)) _output_get_3))
      (`KismetArrayLibrary.Array_Add` (`self.IntArray`) _output_get_3))
    (set `self.Save` false)
    (`KismetArrayLibrary.Array_Remove` _intarray_2)
    (for _array_element_2 _intarray_2
      (set `self.String` (`KismetStringLibrary.BuildString_Int` (`self.String`) " \n" _array_element_2)))
    (else
      ;[0 1 0.3018] Загружаем из сохранки материалы.
      (for _array_element_3 (`KismetStringLibrary.ParseIntoArray` (`self.String`) " \n" false)
        (`KismetArrayLibrary.Array_Add` _intarray (`KismetStringLibrary.Conv_StringToInt` _array_element_3)))
      (`KismetArrayLibrary.Array_Remove` _intarray)))
  (bind _output_get_4 (set `self.ChosenMaterials` (`|GetArrayItem` (`self.RandomMaterials`) (`self.Int`))))
  (for (_array_element_4 _array_index) (`.Random_3_FBC1B23240D51253641D7097DFDE1E31` (break `/NewChristmas/BP/Randomizer/S_PotentialMaterials` _output_get_4))
    (bind _output_get_5 (set `self.Int2` (`|GetArrayItem` (`self.IntArray`) _array_index)))
    (`PrimitiveComponent.SetMaterial` (`StaticMeshActor.StaticMeshComponent` (break `/NewChristmas/BP/Randomizer/S_RandomMaterials` _array_element_4)) (`.IndexMaterial_6_622B93D74E9D80B410BB6C940510CCFE` (break `/NewChristmas/BP/Randomizer/S_RandomMaterials` _array_element_4)) (`|GetArrayItem` (`.Materials_10_81E0B3C0442D85CDEC0549B89F49BAC6` (break `/NewChristmas/BP/Randomizer/S_RandomMaterials` _array_element_4)) _output_get_5))
    (`KismetSystemLibrary.PrintString` (`KismetStringLibrary.Conv_IntToString` _output_get_5) true true (struct :`G` 0.66 :`B` 1.0 :`A` 1.0) 8.0)))

(fn `OnSave`
  (params (JsonObject :type "JSON Structure"))
  (`JSONLibrary.SetValueAsInt` JsonObject "7" (`self.Int`))
  (`JSONLibrary.SetValueAsBool` JsonObject "8" (`self.Save`))
  (`JSONLibrary.SetValueAsInt` JsonObject "9" (`self.Int2`))
  (`JSONLibrary.SetValueAsString` JsonObject "2" (`self.String`)))

(fn `UserConstructionScript`)
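; BP_Lamp_post is a street lamp that switches on at night and off during the morning, day and evening.
; On BeginPlay it finds the first BP_SosedNC actor and reads its day mode to swap the bulb material and set the spotlight intensity.
; EventRefreshGameData re-runs that check after a zero-length delay, so the lamp follows changes in time of day.
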(event `self.ReceiveBeginPlay`
  (bind _staticmesh (`self.StaticMesh`))
  (bind _spotlight (`self.SpotLight`))
  (bind _outactors (`GameplayStatics.GetAllActorsOfClass` "/NewChristmas/Sosed/BP_SosedNC.BP_SosedNC_C"))
  (set `self.Soed` (`|GetArrayItem` _outactors))
  (switch `EDayMode` (`/NewChristmas/Sosed/BP_SosedNC.E_DayMode` (`self.Soed`)) :!label _label
    (:`Morning`
      (`PrimitiveComponent.SetMaterial` _staticmesh 0 "/Game/Objects/Materials/instances/dl_bulb_Off_Inst.dl_bulb_Off_Inst" :!label _label_2)
      (`LightComponent.SetIntensity` _spotlight 0.0))
    (:`Day`
      (goto _label_2))
    (:`Evening`
      (goto _label_2))
    (:`Night`
      (`PrimitiveComponent.SetMaterial` _staticmesh 0 "/Game/Objects/Materials/instances/dl_bulb_On_Inst.dl_bulb_On_Inst")
      (`LightComponent.SetIntensity` _spotlight 100000.0))))

(event `self.EventRefreshGameData`
  (`KismetSystemLibrary.Delay` 0.0)
  (goto _label))

(fn `UserConstructionScript`)
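; BP_NailNC is a nail actor that can be ejected from its position a single time.
; OnEject passes through a DoOnce and teleports the actor, without sweep, along the static mesh's local negative Z axis.
; The travel distance is twice the Z extent of the mesh component's bounds.
; OnIsActionComponent returns true for any component.
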(event `self.OnEject`
  (bind _staticmeshcomponent (`self.StaticMeshComponent`))
  (`/Engine/EditorBlueprintResources/StandardMacros.DoOnce` false
    (:`Completed`
      (`self.K2_SetActorLocation` (+ (* (`KismetMathLibrary.GreaterGreater_VectorRotator` (0.0 0.0 -1.0) (`SceneComponent.K2_GetComponentRotation` _staticmeshcomponent)) (* (.z (`.BoxExtent` (`KismetSystemLibrary.GetComponentBounds` _staticmeshcomponent))) 2.0)) (`self.K2_GetActorLocation`)) false true))))

(fn `OnIsActionComponent`
  (params (Component :type "PrimitiveComponent Object Reference"))
  (returns (Result :type Boolean))
  (return true))

(fn `UserConstructionScript`)
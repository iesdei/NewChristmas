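; Puzzle gate that opens when a BP_PictureHint is placed on its mount and closes when the picture is removed.
; Boom takes the held picture from the player's inventory and fixes it at the mesh transform, with interaction limited to that item.
; Box overlaps and the first picture's Poy event also drive the gate platform.
; The open flag is saved to JSON; loading it restores gate movement and, if open, re-mounts the picture.
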(event `self.ReceiveBeginPlay`
  (bind _outactors (`GameplayStatics.GetAllActorsOfClass` "/NewChristmas/BP/BP_PictureHint.BP_PictureHint_C"))
  (add `/NewChristmas/BP/BP_PictureHint.Poy` (`|GetArrayItem` _outactors) (delegate `GOO`)))

(event `self.OnPostLoad`
  (bind _staticmeshcomponent (`self.StaticMeshComponent`))
  (bind _gate (`self.Gate`))
  (if (`self.Can`)
    (`MovingComponent.SetMovingState` (`/Game/Objects/BP_Objects/BP_PlatformDoor.Platform` _gate) "MS_OPENING")
    (bind _outactors (`GameplayStatics.GetAllActorsOfClass` "/NewChristmas/BP/BP_PictureHint.BP_PictureHint_C"))
    (bind _output (`|GetArrayItem` _outactors))
    (`self.K2_SetActorLocationAndRotation` _output (`SceneComponent.K2_GetComponentLocation` _staticmeshcomponent) (`SceneComponent.K2_GetComponentRotation` _staticmeshcomponent) false true)
    (`FlatComponent.SetMode` (`FlatActor.FlatComponent` _output) "FM_Fixed")
    (else
      (`MovingComponent.SetMovingState` (`/Game/Objects/BP_Objects/BP_PlatformDoor.Platform` _gate) "MS_CLOSING"))))

(event `GOO`
  (`MovingComponent.SetMovingState` (`/Game/Objects/BP_Objects/BP_PlatformDoor.Platform` (`self.Gate`)) "MS_CLOSING" :!label _label)
  (set `self.Can` false))

(event `self.OnLoad`
  (params (JsonObject :type "JSON Structure"))
  (bind _boolvalue (`JSONLibrary.GetValueAsBool` JsonObject "g"))
  (set `self.Can` _boolvalue))

(event `Boom`
  (params (Picture :type "/NewChristmas/BP/BP_PictureHint Object Reference"))
  (bind _staticmeshcomponent (`self.StaticMeshComponent`))
  (`KismetSystemLibrary.PrintString` "Hello")
  (bind _returnvalue (`Human.FindHuman`))
  (bind _returnvalue_2 (`Human.GetInventory` _returnvalue))
  (`Inventory.RemoveObject` _returnvalue_2 (`Inventory.GetCurrentObject` _returnvalue_2))
  (`Human.SetHandsState` _returnvalue "HS_FAST_THROW")
  (`self.K2_SetActorLocationAndRotation` Picture (`SceneComponent.K2_GetComponentLocation` _staticmeshcomponent) (`SceneComponent.K2_GetComponentRotation` _staticmeshcomponent) false true)
  (`FlatComponent.SetMode` (`FlatActor.FlatComponent` Picture) "FM_Fixed")
  (set `self.Can` true)
  (`MovingComponent.SetMovingState` (`/Game/Objects/BP_Objects/BP_PlatformDoor.Platform` (`self.Gate`)) "MS_OPENING" :!label _label_2)
  (set `self.Can` true))

(event `self.Box.OnComponentBeginOverlap`
  (params (OverlappedComponent :type "PrimitiveComponent Object Reference") (OtherActor :type "Actor Object Reference") (OtherComp :type "PrimitiveComponent Object Reference") (OtherBodyIndex :type Integer) (bFromSweep :type Boolean) (SweepResult :type "HitResult Structure (by ref)"))
  (cast `/NewChristmas/BP/BP_PictureHint` OtherActor)
  (goto _label_2))

(event `self.Box.OnComponentEndOverlap`
  (params (OverlappedComponent :type "PrimitiveComponent Object Reference") (OtherActor :type "Actor Object Reference") (OtherComp :type "PrimitiveComponent Object Reference") (OtherBodyIndex :type Integer))
  (cast `/NewChristmas/BP/BP_PictureHint` OtherActor)
  (goto _label))

(fn `OnIsActionComponent`
  (params (Component :type "PrimitiveComponent Object Reference"))
  (returns (Result :type Boolean))
  (bind _returnvalue (`Human.FindHuman`))
  (bind _returnvalue_2 (`Human.GetInventory` _returnvalue))
  (return (== (`GameplayStatics.GetObjectClass` (`Inventory.GetCurrentObject` _returnvalue_2)) "/NewChristmas/BP/BP_PictureHint.BP_PictureHint_C")))

(fn `OnSave`
  (params (JsonObject :type "JSON Structure"))
  (`JSONLibrary.SetValueAsBool` JsonObject "g" (`self.Can`)))

(fn `UserConstructionScript`)
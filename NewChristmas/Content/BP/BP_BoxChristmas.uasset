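; BP_BoxChristmas is a heavy, grabbable Christmas box that takes a random variant from the Random array and saves it.
; With Puk set, post-load rolls separately for mesh, handle and saved Index, so they can mismatch, then clears Puk.
; Otherwise it restores mesh and handle from Index, applying that variant's transform when in hand or inventory.
; Grabbing also applies the transform, and OnSave persists Puk and Index as JSON.
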(event `self.ReceiveBeginPlay`
  (`PrimitiveComponent.SetMassOverrideInKg` (`self.StaticMeshComponent`) "None" 400.0 true))

(event `self.OnLoad`
  (params (JsonObject :type "JSON Structure"))
  (bind _boolvalue (`JSONLibrary.GetValueAsBool` JsonObject "mega"))
  (set `self.puk` _boolvalue)
  (bind _intvalue (`JSONLibrary.GetValueAsInt` JsonObject "integer"))
  (set `self.Index` _intvalue))

(event `self.OnPostLoad`
  (bind _random (`self.Random`))
  (bind _staticmeshcomponent (`self.StaticMeshComponent`))
  (bind _flatcomponent (`self.FlatComponent`))
  (bind _mode (`FlatComponent.Mode` _flatcomponent))
  (bind (_staticmesh _handle _actortransform) (break `/NewChristmas/BP/ST_BoxCh` (`|GetArrayItem` _random (`self.Index`))))
  (bind _returnvalue (`KismetMathLibrary.RandomIntegerInRange` 0 (`KismetArrayLibrary.Array_LastIndex` _random)))
  (bind (_staticmesh_2 _handle_2) (break `/NewChristmas/BP/ST_BoxCh` (`|GetArrayItem` _random _returnvalue)))
  (if (`self.puk`)
    (`StaticMeshComponent.SetStaticMesh` (`self.StaticMeshComponent`) _staticmesh_2)
    (set `FlatComponent.Handle` _handle_2 (`self.FlatComponent`))
    (`KismetSystemLibrary.PrintString` (`KismetSystemLibrary.GetDisplayName` _staticmesh_2) true true (struct :`G` 0.66 :`B` 1.0 :`A` 1.0) 20.0)
    (set `self.puk` false)
    (set `self.Index` _returnvalue)
    (else
      (`StaticMeshComponent.SetStaticMesh` _staticmeshcomponent _staticmesh)
      (set `FlatComponent.Handle` _handle _flatcomponent)
      (if (not (and (`|EnumInequality` _mode "FM_HumanHand") (`|EnumInequality` _mode "FM_Inventory")))
        (`SceneComponent.K2_SetRelativeLocationAndRotation` _staticmeshcomponent (.location _actortransform) (.rotation _actortransform) false true)))))

(event `self.OnGrab`
  (params (Character :type "Actor Object Reference"))
  (`SceneComponent.K2_SetRelativeLocationAndRotation` (`self.StaticMeshComponent`) (.location (`.ActorTransform_9_CC19A13D41691306FC13E9B51F10995A` (break `/NewChristmas/BP/ST_BoxCh` (`|GetArrayItem` (`self.Random`) (`self.Index`))))) (.rotation (`.ActorTransform_9_CC19A13D41691306FC13E9B51F10995A` (break `/NewChristmas/BP/ST_BoxCh` (`|GetArrayItem` (`self.Random`) (`self.Index`))))) false true))

(fn `OnIsActionComponent`
  (params (Component :type "PrimitiveComponent Object Reference"))
  (returns (Result :type Boolean))
  (return true))

(fn `OnSave`
  (params (JsonObject :type "JSON Structure"))
  (`JSONLibrary.SetValueAsBool` JsonObject "mega" (`self.puk`))
  (`JSONLibrary.SetValueAsInt` JsonObject "integer" (`self.Index`)))

(fn `UserConstructionScript`)
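; Crowbar item that the player applies to pry out nails or to place into a BP_WireNeed2 holder.
; Prying plays a use montage with delayed range checks before ejecting the nail, and applying again cancels it.
; A hit frees it from its holder, while grabbing it closes gates of save-flagged BP_WireNeed2 actors.
; Temperature crossing zero swaps hot materials, and save/load tracks the holder, releasing it when none was saved.
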(event `self.ReceiveBeginPlay`
  (bind _returnvalue (`KismetMaterialLibrary.CreateDynamicMaterialInstance` "/Game/Objects/Materials/instances/Hot_Material/metal_noise_hot_Inst.metal_noise_hot_Inst"))
  (bind _returnvalue_2 (`KismetMaterialLibrary.CreateDynamicMaterialInstance` "/Game/Objects/Materials/instances/Hot_Material/red_dark_hot_Inst.red_dark_hot_Inst"))
  (set `self.MaterialsHot` (`|MakeArray` _returnvalue _returnvalue_2)))

(event `self.OnLoad`
  (params (JsonObject :type "JSON Structure"))
  ;[1 1 1] Загрузка из сохранки
  (bind (_stringvalue _returnvalue) (`JSONLibrary.GetValueAsString` JsonObject "Holder"))
  (if _returnvalue
    _
    (elif (`KismetSystemLibrary.IsValid` (`self.Holder`))
      (set `/Game/Objects/BP_Objects/BP_ElectricWires.Crowbar` null (`self.Holder`))
      (set `self.Holder` null)
      (`FlatComponent.SetMode` (`self.FlatComponent`) "FM_Suspend"))))

(event `self.OnPostLoad`
  ;[1 1 1] После загрузки
  (`self.ChangeMaterial`))

(event `self.OnChangeTemperature`
  (params (Old :type "Float (single-precision)") (New :type "Float (single-precision)"))
  ;[1 1 1] Изменения температуры
  (if (or (and (> Old 0.0) (<= New 0.0)) (and (<= Old 0.0) (> New 0.0)))
    (`self.ChangeMaterial`)))

(event `self.ReceiveHit`
  (params (MyComp :type "PrimitiveComponent Object Reference") (Other :type "Actor Object Reference") (OtherComp :type "PrimitiveComponent Object Reference") (bSelfMoved :type Boolean) (HitLocation :type "Vector Structure") (HitNormal :type "Vector Structure") (NormalImpulse :type "Vector Structure") (Hit :type "HitResult Structure (by ref)"))
  ;[1 1 1] Ударился или в него попали чем-то
  (if (`KismetSystemLibrary.IsValid` (`self.Holder`))
    (`FlatComponent.SetMode` (`self.FlatComponent`) "FM_Free")
    (set `/Game/Objects/BP_Objects/BP_ElectricWires.Crowbar` null (`self.Holder`))
    (set `self.Holder` null)))

(event `self.ReceiveTick`
  (params (DeltaSeconds :type "Float (single-precision)")))

(event `ChangeMaterial`
  (bind _staticmeshcomponent (`self.StaticMeshComponent`))
  ;[1 1 1] Изменить метериал
  (if (<= (`self.GetTemperature`) 0.0)
    (`PrimitiveComponent.SetMaterial` _staticmeshcomponent 0 "/Game/Objects/Materials/instances/Hot_Material/metal_noise_hot_Inst.metal_noise_hot_Inst")
    (`PrimitiveComponent.SetMaterial` _staticmeshcomponent 1 "/Game/Objects/Materials/instances/Hot_Material/red_dark_hot_Inst.red_dark_hot_Inst")
    (else
      (`PrimitiveComponent.SetMaterial` _staticmeshcomponent 0 (`|GetArrayItem` (`self.MaterialsHot`)))
      (`PrimitiveComponent.SetMaterial` _staticmeshcomponent 1 (`|GetArrayItem` (`self.MaterialsHot`) 1)))))

(event `self.Apply.OnApply`
  (params (ApplyActor :type "Actor Object Reference") (TraceActor :type "FlatActor Object Reference") (TraceComponent :type "PrimitiveComponent Object Reference"))
  (bind _asbp_nail (cast `/Game/Objects/BP_Objects/BP_Nail` TraceActor)
    (:`then`
      (if (`self.Unpaking?`)
        (bind _returnvalue (`Human.FindHuman` :!label _label))
        (`Character.StopAnimMontage` _returnvalue "/NewChristmas/Player/player_body_use_Montage.player_body_use_Montage")
        (set `self.Unpaking?` false)
        (`Human.SetHandsState` _returnvalue "HS_HOLD")
        (elif (`|EnumEquality` (`FlatComponent.Mode` (`FlatActor.FlatComponent` _asbp_nail)) "FM_Hold")
          (`/Engine/EditorBlueprintResources/StandardMacros.IsValid` _asbp_nail
            (:`Is Valid`
              (set `self.Unpaking?` true)
              (bind _returnvalue_2 (`Human.FindHuman`))
              (`Human.SetHandsState` _returnvalue_2 "HS_WAIT_CHANGE")
              (`|PlayMontage` (`Character.Mesh` _returnvalue_2) "/NewChristmas/Player/player_body_use_Montage.player_body_use_Montage"
                (:`then`
                  (bind _returnvalue_3 (and (<= (`self.GetDistanceTo` _asbp_nail) 160.0) (`self.Unpaking?`)))
                  (if _returnvalue_3
                    (`KismetSystemLibrary.Delay` 1.0)
                    (if _returnvalue_3
                      (`KismetSystemLibrary.Delay` 1.2)
                      (if _returnvalue_3
                        (if _returnvalue_3
                          (`Nail.Eject` _asbp_nail)
                          (else
                            (`Character.StopAnimMontage` _returnvalue_2 "/NewChristmas/Player/player_body_use_Montage.player_body_use_Montage" :!label _label_2)))
                        (else
                          (goto _label_2)))
                      (else
                        (goto _label_2)))
                    (else
                      (goto _label_2)))
                  (`Human.SetHandsState` _returnvalue_2 "HS_HOLD")
                  (set `self.Unpaking?` false))))))))
    (:`CastFailed`
      (bind _asbp_wire_need_2 (cast `/NewChristmas/BP/BP_WireNeed2` TraceActor)
        (:`then`
          (if (not (and (`self.Unpaking?`) (not (== (`self.m_fTemperature`) 0.0))))
            (`/NewChristmas/BP/BP_WireNeed2.HolderCrowbar` _asbp_wire_need_2 self)
            (bind _returnvalue_4 (`Human.FindHuman`))
            (bind _returnvalue_5 (`Human.GetInventory` _returnvalue_4))
            (`Human.SetHandsState` _returnvalue_4 "HS_FAST_THROW")
            (`Inventory.RemoveObject` _returnvalue_5 self)))
        (:`CastFailed`
          (if (`self.Unpaking?`)
            (goto _label)))))))

(event `self.OnGrab`
  (params (Character :type "Actor Object Reference"))
  (bind _outactors (`GameplayStatics.GetAllActorsOfClass` "/NewChristmas/BP/BP_WireNeed2.BP_WireNeed2_C"))
  (for _array_element _outactors
    (if (`/NewChristmas/BP/BP_WireNeed2.Save` _array_element)
      (set `/NewChristmas/BP/BP_WireNeed2.Save` false _array_element)
      (`MovingComponent.SetMovingState` (`/Game/Objects/BP_Objects/BP_PlatformDoor.Platform` (`/NewChristmas/BP/BP_WireNeed2.Gate` _array_element)) "MS_CLOSING"))))

(fn `OnIsActionComponent`
  (params (Component :type "PrimitiveComponent Object Reference"))
  (returns (Result :type Boolean))
  (return true))

(fn `OnSave`
  (params (JsonObject :type "JSON Structure"))
  (if (`KismetSystemLibrary.IsValid` (`self.Holder`))
    (`JSONLibrary.SetValueAsString` JsonObject "Holder" (`KismetSystemLibrary.GetDisplayName` (`self.Holder`)))))

(fn `SetHolder`
  (params (Holder :type "/Game/Objects/BP_Objects/BP_ElectricWires Object Reference"))
  (bind _output_get (set `self.Holder` Holder))
  (if (`KismetSystemLibrary.IsValid` _output_get)
    (`FlatComponent.SetMode` (`self.FlatComponent`) "FM_Fixed")))

(fn `UserConstructionScript`
  (bind _staticmeshcomponent (`self.StaticMeshComponent`))
  (if (<= (`self.GetTemperature`) 0.0)
    (`PrimitiveComponent.SetMaterial` _staticmeshcomponent 0 "/Game/Objects/Materials/instances/metal_noise_dark_Inst.metal_noise_dark_Inst")
    (`PrimitiveComponent.SetMaterial` _staticmeshcomponent 1 "/Game/Objects/Materials/instances/red_dark_wood_Inst.red_dark_wood_Inst")
    (`PrimitiveComponent.SetMaterial` _staticmeshcomponent 2 "/Game/Objects/Materials/instances/metal_noise_Inst.metal_noise_Inst")
    (else
      (`PrimitiveComponent.SetMaterial` _staticmeshcomponent 0 "/Game/Objects/Materials/instances/metal_hot_Inst.metal_hot_Inst")
      (`PrimitiveComponent.SetMaterial` _staticmeshcomponent 1 "/Game/Objects/Materials/instances/metal_hot_Inst.metal_hot_Inst")
      (`PrimitiveComponent.SetMaterial` _staticmeshcomponent 2 "/Game/Objects/Materials/instances/metal_hot_Inst.metal_hot_Inst")
      (`MeshComponent.SetScalarParameterValueOnMaterials` (`self.StaticMeshComponent`) "temperature" (* (`self.GetTemperature`) 15.0)))))
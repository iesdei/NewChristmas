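; Utility pole actor that strings two physical cable wires to another pole referenced by ConnectedPole.
; The construction script sets each cable's end to the matching sphere on that pole, converted into this actor's local space, and can randomize cable gravity scale for varied sag.
; Without a valid connected pole it destroys both cables; the ResetWires branch and event graph do nothing.
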(fn `UserConstructionScript`
  (bind _returnvalue (`KismetMathLibrary.RandomFloatInRange` 20.0 50.0))
  (if (`self.ResetWires`)
    _
    (else
      _))
  (`/Engine/EditorBlueprintResources/StandardMacros.IsValid` (`self.ConnectedPole`)
    (:`Is Valid`
      (set `CableComponent.EndLocation` (`KismetMathLibrary.InverseTransformLocation` (`self.GetTransform`) (`SceneComponent.K2_GetComponentLocation` (`/Game/BP/BP_Pole_Phy_Wire.Sphere1` (`self.ConnectedPole`)))) (`self.Cable1`))
      (set `CableComponent.EndLocation` (`KismetMathLibrary.InverseTransformLocation` (`self.GetTransform`) (`SceneComponent.K2_GetComponentLocation` (`/Game/BP/BP_Pole_Phy_Wire.Sphere2` (`self.ConnectedPole`)))) (`self.Cable2`))
      (if (`self.IsRandomHang`)
        (set `CableComponent.CableGravityScale` _returnvalue (`self.Cable1`))
        (set `CableComponent.CableGravityScale` _returnvalue (`self.Cable2`))))
    (:`Is Not Valid`
      (`ActorComponent.K2_DestroyComponent` (`self.Cable2`))
      (`ActorComponent.K2_DestroyComponent` (`self.Cable1`)))))
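; Item location randomizer that moves a referenced item to a random spot from a list of transforms, driven by save-system callbacks.
; OnPostLoad teleports the item if it is valid and the Save flag is set, then clears the flag so the move does not repeat.
; OnSave and OnLoad persist that flag as a JSON bool, and OnLoad also prints it for debugging.
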(event `self.OnLoad`
  (params (JsonObject :type "JSON Structure"))
  (bind _boolvalue (`JSONLibrary.GetValueAsBool` JsonObject "f"))
  (bind _output_get (set `self.Save` _boolvalue))
  (`KismetSystemLibrary.PrintString` (`KismetStringLibrary.Conv_BoolToString` _output_get) true true (struct :`G` 0.66 :`B` 1.0 :`A` 1.0) 8.0))

(event `self.OnPostLoad`
  (bind _item_locations (`self.Item Locations`))
  (bind _item (`self.Item`))
  (if (`self.Save`)
    (`/Engine/EditorBlueprintResources/StandardMacros.IsValid` _item
      (:`Is Valid`
        (`self.K2_SetActorTransform` _item (`|GetArrayItem` _item_locations (`KismetMathLibrary.RandomIntegerInRange` 0 (`KismetArrayLibrary.Array_LastIndex` _item_locations))) false true)
        (set `self.Save` false)))))

(fn `OnSave`
  (params (JsonObject :type "JSON Structure"))
  (`JSONLibrary.SetValueAsBool` JsonObject "f" (`self.Save`)))

(fn `UserConstructionScript`)
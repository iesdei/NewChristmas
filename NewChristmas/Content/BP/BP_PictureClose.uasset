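; BP_PictureClose is a picture actor that opens a linked gate when something other than the player hits it.
; A hit on its mesh swaps to the closed-picture material, sets the Gate's Platform to OPENING and sets the Again flag.
; The flag saves to and loads from JSON, and post-load reapplies the matching material and gate state.
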(event `self.OnPostLoad`
  (bind _gate (`self.Gate`))
  (if (`self.Again?`)
    (`PrimitiveComponent.SetMaterial` (`self.StaticMeshComponent`) 0 "/NewChristmas/Materials/M_Multi_Pictures_close_Inst.M_Multi_Pictures_close_Inst")
    (`MovingComponent.SetMovingState` (`/Game/Objects/BP_Objects/BP_PlatformDoor.Platform` _gate) "MS_OPENING")
    (else
      (`PrimitiveComponent.SetMaterial` (`self.StaticMeshComponent`) 0 "/Game/Objects/Materials/Multi_Material/M_Multi_Pictures_2_Inst.M_Multi_Pictures_2_Inst")
      (`MovingComponent.SetMovingState` (`/Game/Objects/BP_Objects/BP_PlatformDoor.Platform` _gate) "MS_CLOSE"))))

(event `self.OnLoad`
  (params (JsonObject :type "JSON Structure"))
  (bind _boolvalue (`JSONLibrary.GetValueAsBool` JsonObject "aga"))
  (bind _output_get (set `self.Again?` _boolvalue))
  (`KismetSystemLibrary.PrintString` (`KismetStringLibrary.Conv_BoolToString` _output_get)))

(event `self.ReceiveHit`
  (params (MyComp :type "PrimitiveComponent Object Reference") (Other :type "Actor Object Reference") (OtherComp :type "PrimitiveComponent Object Reference") (bSelfMoved :type Boolean) (HitLocation :type "Vector Structure") (HitNormal :type "Vector Structure") (NormalImpulse :type "Vector Structure") (Hit :type "HitResult Structure (by ref)"))
  (if (and (== MyComp (`self.StaticMeshComponent`)) (!= Other (`GameplayStatics.GetPlayerCharacter` 0)))
    (`PrimitiveComponent.SetMaterial` (`self.StaticMeshComponent`) 0 "/NewChristmas/Materials/M_Multi_Pictures_close_Inst.M_Multi_Pictures_close_Inst")
    (`MovingComponent.SetMovingState` (`/Game/Objects/BP_Objects/BP_PlatformDoor.Platform` (`self.Gate`)) "MS_OPENING")
    (set `self.Again?` true)))

(fn `OnIsActionComponent`
  (params (Component :type "PrimitiveComponent Object Reference"))
  (returns (Result :type Boolean))
  (return true))

(fn `OnSave`
  (params (JsonObject :type "JSON Structure"))
  (`JSONLibrary.SetValueAsBool` JsonObject "aga" (`self.Again?`)))

(fn `UserConstructionScript`)
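; Interactable TV prop with an on/off tumbler switch that also reacts to whether it has electricity.
; Interaction flips the tumbler, which plays or pauses the video and calls ScreenLight (also run at construction) to set spotlight visibility and screen material.
; While switched on, power changes pause or resume the video and swap screen materials.
; Tick randomizes spotlight intensity for screen flicker when powered, zeroing it without power.
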(event `self.ReceiveTick`
  (params (DeltaSeconds :type "Float (single-precision)"))
  (switch `ETumblerState` (`self.GetTumblerState`)
    (:`TUMBLER_ON`
      (if (`self.HasElectricity`)
        (`KismetSystemLibrary.RetriggerableDelay` (`KismetMathLibrary.RandomFloatInRange` 0.0 0.1))
        (`LightComponent.SetIntensity` (`self.Spot`) (`KismetMathLibrary.RandomFloatInRange` 22000.0 45000.0))
        (else
          (`LightComponent.SetIntensity` (`self.Spot`) 0.0))))))

(event `self.OnEventAction`
  (params (ActionMaker :type "Actor Object Reference") (SpecialComponent :type "PrimitiveComponent Object Reference"))
  ;[1 1 1] Comment
  (switch `ETumblerState` (`self.GetTumblerState`)
    (:`TUMBLER_ON`
      (`self.SetTumblerState` "TUMBLER_OFF"))
    (:`TUMBLER_OFF`
      (`self.SetTumblerState` "TUMBLER_ON"))))

(event `self.OnChangeTumblerState`
  (params (NewState :type "ETumblerState Enum" :default "TUMBLER_ON"))
  (bind _video (`self.Video`))
  ;[1 1 1] Comment
  (switch `ETumblerState` NewState
    (:`TUMBLER_ON`
      (`MediaPlayer.Play` _video))
    (:`TUMBLER_OFF`
      (`MediaPlayer.Pause` _video)))
  (`self.ScreenLight`))

(event `self.OnChangeConnection`
  (bind _returnvalue (`self.GetTumblerState`))
  ;[1 1 1] Comment
  (if (`self.HasElectricity`)
    (switch `ETumblerState` _returnvalue
      (:`TUMBLER_ON`
        (`MediaPlayer.Play` (`self.Video`))
        (`PrimitiveComponent.SetMaterial` (`self.StaticMeshComponent`) 1 "/NewChristmas/Materials/ChristmasBULLEVELVEWVQFWQ.ChristmasBULLEVELVEWVQFWQ")))
    (else
      (switch `ETumblerState` _returnvalue
        (:`TUMBLER_ON`
          (`MediaPlayer.Pause` (`self.Video`))
          (`PrimitiveComponent.SetMaterial` (`self.StaticMeshComponent`) 1 "/Game/Objects/Materials/tv_display_off.tv_display_off"))))))

(event `self.ReceiveBeginPlay`
  (`ActorComponent.SetActive` (`self.Spot`) false false)
  (`PrimitiveComponent.SetMassOverrideInKg` (`self.StaticMeshComponent`) "None" 400.0 true))

(fn `OnIsActionComponent`
  (params (Component :type "PrimitiveComponent Object Reference"))
  (returns (Result :type Boolean))
  (return true))

(fn `ScreenLight`
  (bind _spot (`self.Spot`))
  (bind _staticmeshcomponent (`self.StaticMeshComponent`))
  (switch `ETumblerState` (`self.GetTumblerState`)
    (:`TUMBLER_ON`
      (`SceneComponent.SetVisibility` _spot true false)
      (`PrimitiveComponent.SetMaterial` _staticmeshcomponent 1 "/Game/Objects/Materials/tv_display_on.tv_display_on"))
    (:`TUMBLER_OFF`
      (`SceneComponent.SetVisibility` _spot false false)
      (`PrimitiveComponent.SetMaterial` _staticmeshcomponent 1 "/Game/Objects/Materials/instances/Display_Off_Inst.Display_Off_Inst"))))

(fn `UserConstructionScript`
  (`self.ScreenLight`))
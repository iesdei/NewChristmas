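; BP_LocationRondom teleports its referenced Actor to a randomly chosen BP_PontsNC point that shares its Index.
; After load, if the Save flag is set, it gathers matching points, picks one and applies that transform.
; Following a zero-length delay, it copies the point's FlatMode to the Actor's FlatComponent and clears the flag.
; The flag persists through JSON save and load, so a saved placement is not re-randomized.
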(event `self.OnLoad`
  (params (JsonObject :type "JSON Structure"))
  (bind _boolvalue (`JSONLibrary.GetValueAsBool` JsonObject "f"))
  (bind _output_get (set `self.Save` _boolvalue))
  (`KismetSystemLibrary.PrintString` (`KismetStringLibrary.Conv_BoolToString` _output_get) true true (struct :`G` 0.66 :`B` 1.0 :`A` 1.0) 8.0))

(event `self.OnPostLoad`
  (bind _pointsarray (`self.PointsArray`))
  (bind _actor (`self.Actor`))
  (if (`self.Save`)
    (bind _outactors (`GameplayStatics.GetAllActorsOfClass` "/NewChristmas/BP/BP_PontsNC.BP_PontsNC_C"))
    (for _array_element _outactors
      (if (== (`/NewChristmas/BP/BP_PontsNC.Index` _array_element) (`self.Index`))
        (`KismetArrayLibrary.Array_Add` (`self.PointsArray`) _array_element)))
    (`KismetArrayLibrary.Array_Shuffle` _pointsarray)
    (bind _output_get (set `self.CurIndex` (`KismetMathLibrary.RandomIntegerInRange` 0 (`KismetArrayLibrary.Array_LastIndex` _pointsarray))))
    (bind _output (`|GetArrayItem` _pointsarray _output_get))
    (`self.K2_SetActorTransform` _actor (`self.GetTransform` _output) false true)
    (`KismetSystemLibrary.Delay` 0.0)
    (`FlatComponent.SetMode` (`FlatActor.FlatComponent` _actor) (`/NewChristmas/BP/BP_PontsNC.FlatMode` _output))
    (set `self.Save` false)))

(fn `OnSave`
  (params (JsonObject :type "JSON Structure"))
  (`JSONLibrary.SetValueAsBool` JsonObject "f" (`self.Save`)))

(fn `UserConstructionScript`)